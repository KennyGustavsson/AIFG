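; Stationary enemy AI pawn that senses the player, turns to face them and fires on a timer.
; TA vision, hearing and health components switch TAStateMachine between combat, patrol, idle and death states.
; Tick handles combat yaw and firing; death disables senses and credits the player a kill.
; Movement requests from noise, combat and OnWantedMovement call Move, whose MoveToLocation body is disconnected, so the pawn stays put.
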(event OnHealthChange(TAAIHealth)
  (params (CurrentHealthData :type On%20Health%20Change%20Event%20Data%20Structure))
  ;[1 1 1] Health
)

(event OnDeathEvent(TAAIHealth)
  ;[1 1 1] Health
  ;[1 1 1] Die and leave corpse
  (if (not (Variables|Default|GetIsDead))
    (Class|TAStateMachineComponent|ChangeStatefromClass (Variables|Default|GetTAStateMachine) "/Game/_Game/BP/EnemyStates/BP_AI_DeathState.BP_AI_DeathState_C")
    (Variables|Default|SetIsDead true)
    (Default|AddKills (Variables|Default|GetAs%20BP%20Player))
    (Components|Activation|SetActive (Variables|Default|GetTAVision) false false)
    (Components|Activation|SetActive (Variables|Default|GetTAListenening) false false)))

(event OnNoiseHeard(TAListenening)
  (params (Results :type Sound%20Event%20Result%20Structure%20%28by%20ref%29))
  ;[1 1 1] Hearing
  ;[1 1 1] move towards location of sound, if more sound is heard continue towards sound, otherwise return to patrol location after delay
  (if (not (Variables|Default|GetIsDead))
    (if (not (Variables|Default|GetInCombat))
      (Class|TAStateMachineComponent|ChangeStatefromClass (Variables|Default|GetTAStateMachine) "/Game/_Game/BP/EnemyStates/BP_AI_IdleState.BP_AI_IdleState_C")
      (Utilities|Move (.location Results)
        (:Out
          (Class|TAStateMachineComponent|ChangeStatefromClass (Variables|Default|GetTAStateMachine) "/Game/_Game/BP/EnemyStates/BP_AI_PatrolState.BP_AI_PatrolState_C"))))))

(event OnTargetSensed(TAVision)
  (params (Results :type TA%20Vision%20Results%20Structure%20%28by%20ref%29))
  ;[1 1 1] Vision
  (Development|PrintString "I can see you")
  ;[1 1 1] Move in position and fire upon player
  (Class|TAStateMachineComponent|ChangeStatefromClass (Variables|Default|GetTAStateMachine) "/Game/_Game/BP/EnemyStates/BP_AI_CombatState.BP_AI_CombatState_C")
  (Variables|Default|SetInCombat true)
  (Development|PrintString "i am combat"))

(event OnTargetLost(TAVision)
  (params (Results :type TA%20Vision%20Results%20Structure%20%28by%20ref%29))
  ;[1 1 1] Vision
  (Development|PrintString "I Cant see you anymore")
  ;[1 1 1] Combat state if not see target for 10 sec go to patrol state
  (if (not (Variables|Default|GetIsDead))
    (Class|TAStateMachineComponent|ChangeStatefromClass (Variables|Default|GetTAStateMachine) "/Game/_Game/BP/EnemyStates/BP_AI_PatrolState.BP_AI_PatrolState_C")
    (Variables|Default|SetInCombat false)))

(event EventBeginPlay
  ;[1 1 1] Reference to BP_Player
  (bind _asbp_player (Utilities|Casting|CastToBP_Player (Game|Player|GetPlayerPawn 0)))
  (Variables|Default|SetAs%20BP%20Player _asbp_player))

(event EventTick
  (params (DeltaSeconds :type Float%20%28single-precision%29))
  (bind _returnvalue (Game|Player|GetPlayerPawn 0))
  (bind _returnvalue_2 (Transformation|GetActorLocation))
  (bind _returnvalue_3 (Transformation|GetActorLocation _returnvalue))
  ;[1 1 1] Combat behaviour
  (if (not (Variables|Default|GetIsDead))
    (if (Variables|Default|GetInCombat)
      (Variables|Default|SetShootTimer (+ DeltaSeconds (Variables|Default|GetShootTimer)))
      (Transformation|SetActorRotation (Math|Rotator|MakeRotator 0.0 0.0 (.Yaw (Math|Rotator|BreakRotator (Math|Rotator|FindLookatRotation _returnvalue_2 _returnvalue_3)))))
      (if (> (Math|Vector|Distance(Vector) _returnvalue_3 _returnvalue_2) 2.0)
        (if (> (Variables|Default|GetShootTimer) (Variables|Default|GetShootDelay))
          (Audio|PlaySoundatLocation "/Game/Low_Poly_FPS_Pack/Content/Audio/Sound_Cues/Shoot/SC_Shoot_01.SC_Shoot_01" (Transformation|GetActorLocation) "0, 0, 0" 1.0 1.0 0.0 0 0 0)
          (Variables|Default|SetShootTimer 0.0)
          (Class|TAAIWeaponComponent|FireWeapon (Variables|Default|GetTAAIWeapon)))
        (else
          (Utilities|Move (- _returnvalue_3 _returnvalue_2)))))))

(event EventOnWantedMovement
  (params (MoveData :type TA%20Move%20Data%20Structure))
  ;[1 1 1] Movement Handler
  (if (not (Variables|Default|GetIsDead))
    (Utilities|Move (.wanteddestination MoveData))))

(fn ConstructionScript)