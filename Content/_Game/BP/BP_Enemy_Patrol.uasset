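; Patrolling enemy that reacts to sight, sound and health changes, fights the player and credits a kill on death.
; TA component events switch state-machine states between patrol, idle, combat and death.
; Noise or health changes outside combat turn it toward the source or player, and a Tick timer resumes patrol after waiting or losing sight.
; In combat it faces the player, firing on a delay beyond DistanceToShoot and issuing AI moves otherwise.
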(event OnHealthChange(TAAIHealth)
  (params (CurrentHealthData :type On%20Health%20Change%20Event%20Data%20Structure))
  ;[1 1 1] Health
  ;[1 1 1] Rotate towards player
  (if (not (Variables|Default|GetIsDead))
    (if (not (Variables|Default|GetInCombat))
      (Class|TAStateMachineComponent|ChangeStatefromClass (Variables|Default|GetTAStateMachine) "/Game/_Game/BP/EnemyStates/BP_AI_IdleState.BP_AI_IdleState_C")
      (Transformation|SetActorRotation (Math|Rotator|MakeRotator 0.0 0.0 (.Yaw (Math|Rotator|BreakRotator (Math|Rotator|FindLookatRotation (Transformation|GetActorLocation) (Transformation|GetActorLocation (Variables|Default|GetAs%20BP%20Player)))))))
      (Variables|Default|SetWaiting true)
      (Variables|Default|SetWaitingTimer 0.0))))

(event OnDeathEvent(TAAIHealth)
  ;[1 1 1] Health
  (if (not (Variables|Default|GetIsDead))
    ;[1 1 1] Die and leave corpse
    (Class|TAStateMachineComponent|ChangeStatefromClass (Variables|Default|GetTAStateMachine) "/Game/_Game/BP/EnemyStates/BP_AI_DeathState.BP_AI_DeathState_C")
    (Variables|Default|SetIsDead true)
    (Default|AddKills (Variables|Default|GetAs%20BP%20Player))
    (Components|Activation|SetActive (Variables|Default|GetTAVision) false false)
    (Components|Activation|SetActive (Variables|Default|GetTAListenening) false false)))

(event OnNoiseHeard(TAListenening)
  (params (Results :type Sound%20Event%20Result%20Structure%20%28by%20ref%29))
  ;[1 1 1] Hearing
  ;[1 1 1] look towards location of sound, if more sound is heard continue towards sound, otherwise return to patrol location after delay
  (if (not (Variables|Default|GetIsDead))
    (if (not (Variables|Default|GetInCombat))
      (Class|TAStateMachineComponent|ChangeStatefromClass (Variables|Default|GetTAStateMachine) "/Game/_Game/BP/EnemyStates/BP_AI_IdleState.BP_AI_IdleState_C")
      (Transformation|SetActorRotation (Math|Rotator|MakeRotator 0.0 0.0 (.Yaw (Math|Rotator|BreakRotator (Math|Rotator|FindLookatRotation (Transformation|GetActorLocation) (.location Results))))))
      (Variables|Default|SetWaiting true)
      (Variables|Default|SetWaitingTimer 0.0))))

(event OnTargetSensed(TAVision)
  (params (Results :type TA%20Vision%20Results%20Structure%20%28by%20ref%29))
  ;[1 1 1] Vision
  (if (not (Variables|Default|GetIsDead))
    ;[1 1 1] Move in position and fire upon player
    (Variables|Default|SetWaiting false)
    (Variables|Default|SetWaitingTimer 0.0)
    (Class|TAStateMachineComponent|ChangeStatefromClass (Variables|Default|GetTAStateMachine) "/Game/_Game/BP/EnemyStates/BP_AI_CombatState.BP_AI_CombatState_C")
    (Variables|Default|SetInCombat true)))

(event OnTargetLost(TAVision)
  (params (Results :type TA%20Vision%20Results%20Structure%20%28by%20ref%29))
  ;[1 1 1] Vision
  (if (not (Variables|Default|GetIsDead))
    ;[1 1 1] Combat state if not see target for 10 sec go to patrol state
    (Variables|Default|SetWaiting true)
    (Variables|Default|SetWaitingTimer 0.0)
    (Variables|Default|SetInCombat false)))

(event EventBeginPlay
  ;[1 1 1] Begin Play, Reference to BP_Player
  (bind _asbp_player (Utilities|Casting|CastToBP_Player (Game|Player|GetPlayerPawn 0)))
  (Variables|Default|SetAs%20BP%20Player _asbp_player))

(event EventTick
  (params (DeltaSeconds :type Float%20%28single-precision%29))
  ;[1 1 1] Tick
  (if (not (Variables|Default|GetIsDead))
    (if (Variables|Default|GetInCombat)
      (Utilities|Combat DeltaSeconds)
      (else
        ;;[1 1 1] Waiting
        (if (Variables|Default|GetWaiting)
          (if (> (Variables|Default|GetWaitingTimer) (Variables|Default|GetWaitingDelay))
            (Class|TAStateMachineComponent|ChangeStatefromClass (Variables|Default|GetTAStateMachine) "/Game/_Game/BP/EnemyStates/BP_AI_PatrolState.BP_AI_PatrolState_C")
            (Variables|Default|SetWaitingTimer 0.0)
            (else
              (Variables|Default|SetWaitingTimer (+ DeltaSeconds (Variables|Default|GetWaitingTimer))))))))))

(event EventOnWantedMovement
  (params (MoveData :type TA%20Move%20Data%20Structure))
  ;[1 1 1] Movement Handler
  (if (not (Variables|Default|GetIsDead))
    (if (not (Variables|Default|GetInCombat))
      (Utilities|Move (.wanteddestination MoveData)))))

(fn ConstructionScript)