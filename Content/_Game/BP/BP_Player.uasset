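; Player Blueprint for a shooter with run and crouch states, kill-based win tracking and game-over restart or quit.
; TAAI components handle health, death and camera-aimed firing, with each shot also spawning a growing sound event for AI hearing.
; A Crouch subgraph changes Speed, rescales the capsule and lerps camera height through timelines.
; AddKills counts down remaining enemies to set WinState; BeginPlay shows the kill-count widget, and Y applies self-damage.
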(event OnHealthChange(TAAIHealth)
  (params (CurrentHealthData :type On%20Health%20Change%20Event%20Data%20Structure))
  ;[1 1 1] Hook to Health..
  (Variables|Default|SetHealth (Math|Conversions|ToFloat(Integer) (.currenthealth CurrentHealthData))))

(event OnDeathEvent(TAAIHealth)
  ;[1 1 1] Death Event
  (Variables|Default|SetGameOver? true)
  (Class|TAPlayer|ActiveInput false)
  (Class|TAPlayer|ZeroInputVector))

(event Custom|AddKills
  ;[1 1 1] Kill Count
  (Variables|Default|SetKillCount (+ (Variables|Default|GetKillCount) 1))
  (Variables|Default|SetEnemy%20Left (- (Variables|Default|GetEnemy%20Left) 1))
  (if (== (Variables|Default|GetEnemy%20Left) 0)
    (Variables|Default|SetWinState? true)))

(event EventBeginPlay
  ;[1 1 1] Creates Widget
  (bind _returnvalue (UserInterface|CreateWidget "/Game/_Game/BP/W_KillCount.W_KillCount_C" 0 self))
  (UserInterface|Viewport|AddtoViewport _returnvalue 0))

(event Input|ActionEvents|InputActionCrouch
  (params (Key :type Key%20Structure :default "None"))
  ;[1 1 1] Crouch
  (:Pressed
    (Character|Crouch :!label _label))
  (:Released
    (goto _label execute2)))

(event Input|KeyboardEvents|Y
  (params (Key :type Key%20Structure :default "None"))
  (:Pressed
    (Class|TAAIHealthComponent|Damage (Variables|Default|GetTAAIHealth) 25)))

(event Input|MouseEvents|RightMouseButton
  (params (Key :type Key%20Structure :default "None")))

(event Input|KeyboardEvents|W
  (params (Key :type Key%20Structure :default "None"))
  (:Pressed
    (if (not (Variables|Default|GetIsDead))
      (Variables|Default|SetisRunning true)))
  (:Released
    (Variables|Default|SetisRunning false)))

(event Input|MouseEvents|LeftMouseButton
  (params (Key :type Key%20Structure :default "None")))

(event Input|MouseEvents|LeftMouseButton
  (params (Key :type Key%20Structure :default "None"))
  (bind _returnvalue (Transformation|GetActorLocation))
  (:Pressed
    (if (not (Variables|Default|GetIsDead))
      (Variables|Default|SetisShooting true)
      (Class|TAAIWeaponComponent|FireWeaponfromCameraComponent (Variables|Default|GetTAAIWeapon) (Variables|Default|GetMyCamera))
      (Class|SoundEvent|SpawnSoundEvent (Utilities|Struct|MakeSoundEventData self _returnvalue 2.0 8e+02 5e+02 false))
      (Audio|PlaySoundatLocation "/Game/Low_Poly_FPS_Pack/Content/Audio/Sound_Cues/Shoot/SC_Shoot_01.SC_Shoot_01" _returnvalue "0, 0, 0" 1.0 1.0 0.0 0 0 0)))
  (:Released
    (Variables|Default|SetisShooting false)))

(event Input|KeyboardEvents|R
  (params (Key :type Key%20Structure :default "None"))
  (:Pressed
    (if (Variables|Default|GetGameOver?)
      (Game|OpenLevel(byName) "MainMap1")
      (Variables|Default|SetGameOver? false))))

(event Input|KeyboardEvents|Q
  (params (Key :type Key%20Structure :default "None"))
  (:Pressed
    (if (Variables|Default|GetGameOver?)
      (Game|QuitGame 0 "Quit" false))))

(fn ConstructionScript
  (Variables|Default|SetRelative%20Location (Variables|/Script/Engine.SceneComponent|GetRelativeLocation (Variables|Default|GetMyCamera))))